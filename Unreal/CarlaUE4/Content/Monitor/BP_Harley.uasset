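; BP_Harley is a Harley vehicle Blueprint that displays turn and hazard signals on its front and rear indicator components.
; It overrides SetSignal, calling the parent and then switching on Off, Right, Left or Emergency.
; Each state swaps the four indicators between blink and transparent materials, so the Blueprint needs no Tick or timer logic.
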(event EventBeginPlay
  (|CallParentFunction) ; This node is disabled and will not be called.\nDrag off pins to build functionality.
)

(event Collision|EventActorBeginOverlap
  (params (OtherActor :type Actor%20Object%20Reference))
  (|CallParentFunction OtherActor) ; This node is disabled and will not be called.\nDrag off pins to build functionality.
)

(event EventTick
  (params (DeltaSeconds :type Float%20%28single-precision%29))
  (|CallParentFunction DeltaSeconds) ; This node is disabled and will not be called.\nDrag off pins to build functionality.
)

(event EventSetSignal
  (params (Signal :type EVehicleSignalState%20Enum :default "Off"))
  (|CallParentFunction Signal)
  (switch Utilities|FlowControl|Switch|SwitchonEVehicleSignalState Signal
    (:Off
      (Rendering|Material|SetMaterial (Variables|Default|GetLeftSignalFront) 0 "/Game/Monitor/Transparent_M.Transparent_M")
      (Rendering|Material|SetMaterial (Variables|Default|GetLeftSignalRear) 0 "/Game/Monitor/Transparent_M.Transparent_M")
      (Rendering|Material|SetMaterial (Variables|Default|GetRightSignalFront) 0 "/Game/Monitor/Transparent_M.Transparent_M")
      (Rendering|Material|SetMaterial (Variables|Default|GetRightSignalRear) 0 "/Game/Monitor/Transparent_M.Transparent_M"))
    (:Right
      (Rendering|Material|SetMaterial (Variables|Default|GetRightSignalFront) 0 "/Game/Monitor/Blink_M.Blink_M")
      (Rendering|Material|SetMaterial (Variables|Default|GetRightSignalRear) 0 "/Game/Monitor/Blink_M.Blink_M")
      (Rendering|Material|SetMaterial (Variables|Default|GetLeftSignalFront) 0 "/Game/Monitor/Transparent_M.Transparent_M")
      (Rendering|Material|SetMaterial (Variables|Default|GetLeftSignalRear) 0 "/Game/Monitor/Transparent_M.Transparent_M"))
    (:Left
      (Rendering|Material|SetMaterial (Variables|Default|GetLeftSignalFront) 0 "/Game/Monitor/Blink_M.Blink_M")
      (Rendering|Material|SetMaterial (Variables|Default|GetLeftSignalRear) 0 "/Game/Monitor/Blink_M.Blink_M")
      (Rendering|Material|SetMaterial (Variables|Default|GetRightSignalFront) 0 "/Game/Monitor/Transparent_M.Transparent_M")
      (Rendering|Material|SetMaterial (Variables|Default|GetRightSignalRear) 0 "/Game/Monitor/Transparent_M.Transparent_M"))
    (:Emergency
      (Rendering|Material|SetMaterial (Variables|Default|GetLeftSignalFront) 0 "/Game/Monitor/Blink_M.Blink_M")
      (Rendering|Material|SetMaterial (Variables|Default|GetLeftSignalRear) 0 "/Game/Monitor/Blink_M.Blink_M")
      (Rendering|Material|SetMaterial (Variables|Default|GetRightSignalFront) 0 "/Game/Monitor/Blink_M.Blink_M")
      (Rendering|Material|SetMaterial (Variables|Default|GetRightSignalRear) 0 "/Game/Monitor/Blink_M.Blink_M"))))

(fn ConstructionScript
  (|CallParentFunction))